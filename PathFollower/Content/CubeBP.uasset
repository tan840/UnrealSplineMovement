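; CubeBP is an actor that travels along the spline of a SplinePathBP actor found in the level at BeginPlay.
; MoveMesh plays a timeline at a rate of 1/TimeToComplete, using its track to interpolate distance over the spline's length.
; Each update sets the actor's transform from that distance, taking location in world space but rotation in the spline's local space.
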(event `self.ReceiveBeginPlay`
  (`self.EnableInput` (`GameplayStatics.GetPlayerController` 0))
  (`KismetSystemLibrary.PrintString` "Begin" true true (struct :`G` 0.66 :`B` 1.0 :`A` 1.0) 10.0)
  (bind _returnvalue (`GameplayStatics.GetActorOfClass` "/Game/SplinePathBP.SplinePathBP_C"))
  (set `self.splineRef` _returnvalue)
  (`self.MoveMesh`))

(event `self.ReceiveTick`
  (params (DeltaSeconds :type "Float (single-precision)")))

(event `MoveMesh`
  (bind _spline (`/Game/SplinePathBP.Spline` (`self.splineRef`)))
  (`TimelineComponent.SetPlayRate` (`self.Timeline T`) (/ 1.0 (`self.TimeToComplete`)))
  (bind (_direction _movetrack) (`Timeline|Timeline T`)
    (:`Update`
      (bind _returnvalue (`KismetMathLibrary.Lerp` 0.0 (`SplineComponent.GetSplineLength` (`/Game/SplinePathBP.Spline` (`self.splineRef`))) _movetrack))
      (`self.K2_SetActorTransform` (`KismetMathLibrary.MakeTransform` (`SplineComponent.GetLocationAtDistanceAlongSpline` _spline _returnvalue "World") (`SplineComponent.GetRotationAtDistanceAlongSpline` _spline _returnvalue "Local"))))))

(fn `UserConstructionScript`)